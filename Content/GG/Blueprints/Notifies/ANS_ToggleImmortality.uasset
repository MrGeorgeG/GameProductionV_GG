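; Anim notify state, shown as "Immortal", that makes the animated mesh's owner immortal for the duration of the notify window.
; On begin it sends the enable immortality message and on end the disable message.
; Both calls go through the BPI_CanBeImmortal interface, only when the owning actor implements it, so the notify stays decoupled from specific actor classes.
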(fn ReceivedNotifyEnd
  (params (MeshComp :type Skeletal%20Mesh%20Component%20Object%20Reference) (Animation :type Anim%20Sequence%20Base%20Object%20Reference))
  (bind _returnvalue (Components|GetOwner MeshComp))
  (if (Utilities|DoesObjectImplementInterface _returnvalue "/Game/GG/Blueprints/Interfaces/BPI_CanBeImmortal.BPI_CanBeImmortal_C")
    (Class|BPICanbeImmortal|DisableImmortality(Message) _returnvalue)
    (return false)))

(fn GetNotifyName
  (return "Immortal"))

(fn ReceivedNotifyBegin
  (params (MeshComp :type Skeletal%20Mesh%20Component%20Object%20Reference) (Animation :type Anim%20Sequence%20Base%20Object%20Reference) (TotalDuration :type Float%20%28single-precision%29))
  (bind _returnvalue (Components|GetOwner MeshComp))
  (if (Utilities|DoesObjectImplementInterface _returnvalue "/Game/GG/Blueprints/Interfaces/BPI_CanBeImmortal.BPI_CanBeImmortal_C")
    (Class|BPICanbeImmortal|EnableImmortality(Message) _returnvalue)
    (return false)))